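; BP_PotatoEaterCharacter_2 is a potato eater character Blueprint whose only graph logic animates changes to the actor's size.
; The SetScale event stores the current scale and a uniform target, then restarts a timeline with its play rate set from AnimationTotalTime.
; Each timeline update applies an exponential ease-in-out between the two scales.
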(event `self.ReceiveBeginPlay`)

(event `self.ReceiveActorBeginOverlap`
  (params (OtherActor :type "Actor Object Reference")))

(event `self.ReceiveTick`
  (params (DeltaSeconds :type "Float (single-precision)")))

(event `self.SetScale`
  (params (scale :type "Float (single-precision)"))
  (set `self.TargetScale` (`KismetMathLibrary.Conv_DoubleToVector` scale))
  (set `self.StartingScale` (`self.GetActorScale3D`))
  (`TimelineComponent.SetPlayRate` (`self.UpdateScaleTimeline`) (/ 1.0 (`self.AnimationTotalTime`)))
  (bind (_direction _0_1) (`Timeline|UpdateScaleTimeline` :!via `PlayFromStart`)
    (:`Update`
      (`self.SetActorScale3D` (`|EaseFunction` "ExpoInOut" _0_1 (`self.StartingScale`) (`self.TargetScale`))))))

(fn `UserConstructionScript`)